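; Player controller that turns Enhanced Input actions into character movement, camera look, jumping and sprinting.
; On BeginPlay it adds the base mapping context and caches the controlled pawn as a Character for later actions.
; Movement rotates the character's forward vector by the input direction, while look applies scaled yaw and pitch.
; Sprint switches the character's max walk speed between a fast and a normal value.
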(event `self.ReceiveBeginPlay`
  (`EnhancedInputSubsystemInterface.AddMappingContext` (subsystem `EnhancedInputLocalPlayerSubsystem`) "/Game/Inputs/IMC_Base.IMC_Base" 0 (struct))
  (bind _ascharacter (cast `Character` (`self.K2_GetPawn`)))
  (set `self.MyChar` _ascharacter))

(event `EnhancedInput|/Game/Inputs/IA_Move`
  (params (ActionValue :type "Vector2D Structure") (ElapsedSeconds :type "Float (double-precision)") (TriggeredSeconds :type "Float (double-precision)") (InputAction :type "InputAction Object Reference" :default "/Game/Inputs/IA_Move.IA_Move"))
  (:`Triggered`
    (`Pawn.AddMovementInput` (`self.MyChar`) (`KismetMathLibrary.GreaterGreater_VectorRotator` (`KismetMathLibrary.Conv_RotatorToVector` (`self.K2_GetActorRotation` (`self.MyChar`))) (`KismetMathLibrary.Conv_VectorToRotator` (`KismetMathLibrary.Conv_Vector2DToVector` ActionValue))) 1.0 false)))

(event `EnhancedInput|/Game/Inputs/IA_Look`
  (params (ActionValue :type "Vector2D Structure") (ElapsedSeconds :type "Float (double-precision)") (TriggeredSeconds :type "Float (double-precision)") (InputAction :type "InputAction Object Reference" :default "/Game/Inputs/IA_Look.IA_Look"))
  (bind (_x _y) (`KismetMathLibrary.BreakVector2D` ActionValue))
  (:`Triggered`
    (`self.AddYawInput` (* _x 0.4))
    (`self.AddPitchInput` (* _y 0.4))))

(event `EnhancedInput|/Game/Inputs/IA_Jump`
  (params (ActionValue :type "Float (double-precision)") (ElapsedSeconds :type "Float (double-precision)") (TriggeredSeconds :type "Float (double-precision)") (InputAction :type "InputAction Object Reference" :default "/Game/Inputs/IA_Jump.IA_Jump"))
  (:`Triggered`
    (`Character.Jump` (`self.MyChar`))))

(event `EnhancedInput|/Game/Inputs/IA_Sprint`
  (params (ActionValue :type "Float (double-precision)") (ElapsedSeconds :type "Float (double-precision)") (TriggeredSeconds :type "Float (double-precision)") (InputAction :type "InputAction Object Reference" :default "/Game/Inputs/IA_Sprint.IA_Sprint"))
  (bind _charactermovement (`Character.CharacterMovement` (`self.MyChar`)))
  (:`Triggered`
    (set `CharacterMovementComponent.MaxWalkSpeed` 1000.0 _charactermovement :!label _label))
  (:`Started`
    (goto _label))
  (:`Canceled`
    (set `CharacterMovementComponent.MaxWalkSpeed` 600.0 _charactermovement :!label _label_2))
  (:`Completed`
    (goto _label_2)))

(fn `UserConstructionScript`)